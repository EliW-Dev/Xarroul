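; Player ship Blueprint that drives the visual effects of its left and right engines from input.
; Thrust updates scale the input value, clamp it to a minimum and write it to the EngineThrust variable on both effects.
; Rotation updates pass the input rotation to both engines' EngineRotation vector.
; An unconnected copy of the thrust update never runs, and the construction script is empty.
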(event `self.OnInputThrustValueUpdated`
  (bind _returnvalue (`KismetMathLibrary.FMax` (* (`self.InputThrustValue`) 100.0) 50.0))
  ;[1 1 1] Ship Engine FX
  (`NiagaraComponent.SetVariableFloat` (`self.LeftEngine`) "EngineThrust" _returnvalue)
  (`NiagaraComponent.SetVariableFloat` (`self.RightEngine`) "EngineThrust" _returnvalue))

(event `self.OnInputRotValueUpdated`
  (bind _inputrotationvalue (`self.InputRotationValue`))
  ;[1 1 1] Ship Engine FX
  (`NiagaraComponent.SetVariableVec3` (`self.LeftEngine`) "EngineRotation" (`KismetMathLibrary.MakeVector` _inputrotationvalue))
  (`NiagaraComponent.SetVariableVec3` (`self.RightEngine`) "EngineRotation" (`KismetMathLibrary.MakeVector` _inputrotationvalue)))

(fn `UserConstructionScript`)